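; Base actor for grabbable objects with a changeable, replicated color.
; Interacting passes the object to the interacting character's BPGrabbingComponent to be grabbed.
; Server_ChangeColor sets Color, whose OnRep builds a dynamic instance of M_FlatCol1, sets its Base Color parameter and applies it to the static mesh.
; An older ObjectColor rep function remains, with its preset color selection left unused.
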(event `/Game/Core/Interfaces/BPI_Interact.Interact`
  (params (CharacterRef :type "/Game/ThirdPerson/Blueprints/BP_ThirdPersonCharacter Object Reference"))
  ; Grab
  (`/Game/Core/Components/BP_GrabbingComponent.GrabObject` (`/Game/ThirdPerson/Blueprints/BP_ThirdPersonCharacter.BP_GrabbingComponent` CharacterRef) self))

(event `Server_ChangeColor`
  (params (LinearColor :type "LinearColor Structure"))
  ; Change Item Color
  (set `self.Color` LinearColor))

(fn `OnRep_Color`
  (bind _staticmesh (`self.StaticMesh`))
  (bind _returnvalue (`PrimitiveComponent.CreateDynamicMaterialInstance` _staticmesh 0 "/Game/Core/Materials/M_FlatCol1.M_FlatCol1" "None"))
  (`MaterialInstanceDynamic.SetVectorParameterValue` _returnvalue "Base Color" (`self.Color`))
  (`PrimitiveComponent.SetMaterial` _staticmesh 0 _returnvalue))

(fn `OnRep_ObjectColor`
  (`KismetMaterialLibrary.SetVectorParameterValue` null "Base Color" (`self.Color`)))

(fn `UserConstructionScript`)