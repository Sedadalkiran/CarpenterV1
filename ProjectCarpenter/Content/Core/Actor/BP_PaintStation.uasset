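; BP_PaintStation is a paint station actor that tracks a grabbable object placed inside its Box trigger.
; On the server, overlap begin stores a BP_BaseGrapObject in ObjectRefForPaint if that slot holds no valid object.
; Overlap end clears the reference when any grab object leaves, even if it is not the stored one.
; The file contains no painting logic, only this reference tracking.
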(event `self.ReceiveBeginPlay`)

(event `self.Box.OnComponentBeginOverlap`
  (params (OverlappedComponent :type "PrimitiveComponent Object Reference") (OtherActor :type "Actor Object Reference") (OtherComp :type "PrimitiveComponent Object Reference") (OtherBodyIndex :type Integer) (bFromSweep :type Boolean) (SweepResult :type "HitResult Structure (by ref)"))
  (`/Engine/EditorBlueprintResources/ActorMacros.Switch Has Authority`
    (:`Authority`
      (bind _asbp_base_grap_object (cast `/Game/Core/Actor/BP_BaseGrapObject` OtherActor))
      (`/Engine/EditorBlueprintResources/StandardMacros.IsValid` (`self.ObjectRefForPaint`)
        (:`Is Not Valid`
          (set `self.ObjectRefForPaint` _asbp_base_grap_object))))))

(event `self.Box.OnComponentEndOverlap`
  (params (OverlappedComponent :type "PrimitiveComponent Object Reference") (OtherActor :type "Actor Object Reference") (OtherComp :type "PrimitiveComponent Object Reference") (OtherBodyIndex :type Integer))
  (`/Engine/EditorBlueprintResources/ActorMacros.Switch Has Authority`
    (:`Authority`
      (cast `/Game/Core/Actor/BP_BaseGrapObject` OtherActor)
      (set `self.ObjectRefForPaint` null))))

(fn `UserConstructionScript`
  (`parent.UserConstructionScript`))