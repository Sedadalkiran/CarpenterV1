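; BP_CarvingMachine is an interactable production machine that lets a player pick an item to produce.
; Interact sets the character as owner and toggles WBP_OrderWidget, switching cursor, move/look input and input mode.
; A selection in the widget goes through the player character's ServerRequestItemSpawn, passing the item and machine.
; RequestSpawn spawns the item's class at SpawnPoint and marks it Produced.
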(event `/Game/Core/Interfaces/BPI_Interact.Interact`
  (params (CharacterRef :type "/Game/ThirdPerson/Blueprints/BP_ThirdPersonCharacter Object Reference"))
  (bind _returnvalue (`GameplayStatics.GetPlayerController` 0))
  (bind _returnvalue_2 (`Pawn.GetController` CharacterRef))
  ; Create UI when Interact
  (`self.SetOwner` CharacterRef)
  (`/Engine/EditorBlueprintResources/StandardMacros.IsValid` (`self.WidgetRef`)
    (:`Is Valid`
      (`Widget.RemoveFromParent` (`self.WidgetRef`))
      (set `self.WidgetRef` null)
      (`Controller.SetIgnoreMoveInput` _returnvalue_2 false)
      (`Controller.SetIgnoreLookInput` _returnvalue_2 false)
      (set `PlayerController.bShowMouseCursor` false _returnvalue)
      (`WidgetBlueprintLibrary.SetInputMode_GameOnly` _returnvalue))
    (:`Is Not Valid`
      (bind _returnvalue_3 (`|CreateWidget` "/Game/Core/Widgets/WBP_OrderWidget.WBP_OrderWidget_C"))
      (set `self.WidgetRef` _returnvalue_3)
      (`UserWidget.AddToViewport` _returnvalue_3 0)
      (add `/Game/Core/Widgets/WBP_OrderWidget.ED_CallItemSelected` _returnvalue_3 (delegate `Production`))
      (bind _returnvalue_4 (`Widget.GetOwningPlayer` _returnvalue_3))
      (set `PlayerController.bShowMouseCursor` true _returnvalue_4)
      (`Controller.SetIgnoreMoveInput` _returnvalue_4 true)
      (`Controller.SetIgnoreLookInput` _returnvalue_4 true)
      (`WidgetBlueprintLibrary.SetInputMode_GameAndUIEx` _returnvalue_4 null))))

(event `Production`
  (params (SelectedItem :type "/Game/Core/Data/BP_ItemData Object Reference"))
  ; On Produce
  (bind _asbp_third_person_character (cast `/Game/ThirdPerson/Blueprints/BP_ThirdPersonCharacter` (`UserWidget.GetOwningPlayerPawn` (stale `/Game/Core/Interfaces/BPI_Interact.Interact` _returnvalue_3))))
  (set `self.Selected Item` SelectedItem)
  (`/Game/ThirdPerson/Blueprints/BP_ThirdPersonCharacter.Server_RequestItemSpawn` _asbp_third_person_character SelectedItem self))

(event `RequestSpawn`
  (params (Item :type "/Game/Core/Data/BP_ItemData Object Reference"))
  (bind _returnvalue_location (`KismetMathLibrary.BreakTransform` (`SceneComponent.K2_GetComponentToWorld` (`self.SpawnPoint`))))
  ; Spawn
  (bind _returnvalue (`|SpawnActorFromClass` (`/Game/Core/Data/BP_ItemData.ItemClassRef` Item) (`KismetMathLibrary.MakeTransform` _returnvalue_location) "Undefined" "MultiplyWithRoot" null null))
  (`/Engine/EditorBlueprintResources/StandardMacros.IsValid` _returnvalue
    (:`Is Valid`
      (set `/Game/Core/Actor/BP_BaseGrapObject.State` (struct :`GameplayTags` (struct :`(TagName` "Item.State.Produced"))) _returnvalue))))

(fn `UserConstructionScript`)