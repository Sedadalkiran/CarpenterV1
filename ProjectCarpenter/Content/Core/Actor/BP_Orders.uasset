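; BP_Orders is an interactable actor that opens and closes an on-screen list of the game's active orders.
; Interact toggles on a stored widget reference, switching input mode and blocking or restoring the character's move and look input.
; On opening, it reads ActiveOrders from BP_NewGameState and adds one slot widget per order showing its item type, with the color text left empty.
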(event `/Game/Core/Interfaces/BPI_Interact.Interact`
  (params (CharacterRef :type "/Game/ThirdPerson/Blueprints/BP_ThirdPersonCharacter Object Reference"))
  (bind _returnvalue (`Pawn.GetController` CharacterRef))
  (bind _returnvalue_2 (`Pawn.GetController` CharacterRef))
  (`/Engine/EditorBlueprintResources/StandardMacros.IsValid` (`self.WidgetRef`)
    (:`Is Valid`
      ; Remove Widget
      (`WidgetBlueprintLibrary.SetInputMode_GameOnly` (`GameplayStatics.GetPlayerController` 0))
      (`Controller.SetIgnoreMoveInput` _returnvalue false)
      (`Controller.SetIgnoreLookInput` _returnvalue false)
      (`Widget.RemoveFromParent` (`self.WidgetRef`))
      (set `self.WidgetRef` null))
    (:`Is Not Valid`
      ; Create widget
      (bind _asbp_new_game_state (cast `/Game/ThirdPerson/Blueprints/BP_NewGameState` (`GameplayStatics.GetGameState`)))
      (bind _returnvalue_3 (`|CreateWidget` "/Game/Core/Widgets/WBP_ActiveOrders.WBP_ActiveOrders_C"))
      (`UserWidget.AddToViewport` _returnvalue_3 0)
      (set `self.WidgetRef` _returnvalue_3)
      (`WidgetBlueprintLibrary.SetInputMode_GameAndUIEx` (`GameplayStatics.GetPlayerController` 0) (`self.WidgetRef`))
      (`Controller.SetIgnoreMoveInput` _returnvalue_2 true)
      (`Controller.SetIgnoreLookInput` _returnvalue_2 true)
      (for _array_element (`/Game/ThirdPerson/Blueprints/BP_NewGameState.ActiveOrders` _asbp_new_game_state)
        (bind _returnvalue_4 (`|CreateWidget` "/Game/Core/Widgets/WBP_ActiveOrdersSlot.WBP_ActiveOrdersSlot_C"))
        (`TextBlock.SetText` (`/Game/Core/Widgets/WBP_ActiveOrdersSlot.Type` _returnvalue_4) (`KismetTextLibrary.Conv_ObjectToText` (`.ItemType_14_286166BE4B12B5C9E4E936BFFF249DCA` (break `/Game/Core/Data/S_OrderItemData` _array_element))))
        (`TextBlock.SetText` (`/Game/Core/Widgets/WBP_ActiveOrdersSlot.Color` _returnvalue_4) "")
        (`PanelWidget.AddChild` (`/Game/Core/Widgets/WBP_ActiveOrders.OrderList` _returnvalue_3) _returnvalue_4)))))

(fn `UserConstructionScript`
  (`parent.UserConstructionScript`))