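; Delivery area actor that pays the team budget when a produced, painted item is brought into it to fill an order.
; On Box overlap, the server compares the BP_BaseGrapObject's class, color and state tags against BP_GameState's ActiveOrders.
; A full match pays full reward, removes the order and destroys the item.
; Each wrong-color class match checked before that pays half, leaving order and item in place.
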(event `self.Box.OnComponentBeginOverlap`
  (params (OverlappedComponent :type "PrimitiveComponent Object Reference") (OtherActor :type "Actor Object Reference") (OtherComp :type "PrimitiveComponent Object Reference") (OtherBodyIndex :type Integer) (bFromSweep :type Boolean) (SweepResult :type "HitResult Structure (by ref)"))
  (`/Engine/EditorBlueprintResources/ActorMacros.Switch Has Authority`
    (:`Authority`
      (bind _asbp_base_grap_object (cast `/Game/Core/Actor/BP_BaseGrapObject` OtherActor))
      (bind _asbp_game_state (cast `/Game/ThirdPerson/Blueprints/BP_GameState` (`GameplayStatics.GetGameState`)))
      (bind _activeorders (`/Game/ThirdPerson/Blueprints/BP_GameState.ActiveOrders` _asbp_game_state))
      (for _array_element _activeorders
        (bind (_itemtype _ordercolor) (break `/Game/Core/Data/S_OrderItemData` _array_element))
        (bind _returnvalue (== (`/Game/Core/Data/BP_ItemData.ItemClassRef` _itemtype) (`GameplayStatics.GetObjectClass` _asbp_base_grap_object)))
        (bind _state (`/Game/Core/Actor/BP_BaseGrapObject.State` _asbp_base_grap_object))
        (bind _returnvalue_2 (`BlueprintGameplayTagLibrary.HasTag` _state (struct :`TagName` "Item.State.Produced")))
        (bind _returnvalue_3 (`BlueprintGameplayTagLibrary.HasTag` _state (struct :`TagName` "Item.State.Painted")))
        (if (and (== _ordercolor (`/Game/Core/Actor/BP_BaseGrapObject.Color` _asbp_base_grap_object)) _returnvalue _returnvalue_2 _returnvalue_3)
          (set `/Game/ThirdPerson/Blueprints/BP_GameState.TotalBudget` (+ (`/Game/ThirdPerson/Blueprints/BP_GameState.TotalBudget` _asbp_game_state) 100.0) _asbp_game_state)
          (bind _returnvalue_4 (`KismetArrayLibrary.Array_RemoveItem` _activeorders))
          (if _returnvalue_4
            (`self.K2_DestroyActor` _asbp_base_grap_object)
            (break))
          (elif (and _returnvalue_2 _returnvalue_3 _returnvalue)
            (set `/Game/ThirdPerson/Blueprints/BP_GameState.TotalBudget` (+ (`/Game/ThirdPerson/Blueprints/BP_GameState.TotalBudget` _asbp_game_state) 50.0) _asbp_game_state)))))))

(fn `UserConstructionScript`)