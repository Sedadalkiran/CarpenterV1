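; BP_PaintCup is an interactable paint cup that lets a character request its color at an associated paint station.
; On BeginPlay it tints its static mesh with a dynamic instance of M_FlatCol1, setting Base Color from its Color variable.
; Interact passes Mystation and Color to ServerRequestPaint on the interacting character, which owns the paint request.
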(event `self.ReceiveBeginPlay`
  (bind _returnvalue (`PrimitiveComponent.CreateDynamicMaterialInstance` (`self.StaticMesh`) 0 "/Game/Core/Materials/M_FlatCol1.M_FlatCol1" "None"))
  (`MaterialInstanceDynamic.SetVectorParameterValue` _returnvalue "Base Color" (`self.Color`))
  (`PrimitiveComponent.SetMaterial` (`self.StaticMesh`) 0 _returnvalue))

(event `/Game/Core/Interfaces/BPI_Interact.Interact`
  (params (CharacterRef :type "/Game/ThirdPerson/Blueprints/BP_ThirdPersonCharacter Object Reference"))
  (`/Game/ThirdPerson/Blueprints/BP_ThirdPersonCharacter.Server_RequestPaint` CharacterRef (`self.Mystation`) (`self.Color`)))

(fn `UserConstructionScript`)