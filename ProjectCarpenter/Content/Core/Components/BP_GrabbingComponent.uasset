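; Actor component on the third-person character that lets it grab, carry and drop a nearby object.
; Grab requests go to a server event that checks range, sets owner and held state, and disables the mesh's physics and collision.
; A looping timer interpolates the object toward the character's GrabPoint on authority, then attaches it when close.
; DropItem detaches and restores physics on authority only; ServerDropItem and OnRep_HeldItem are empty.
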(event `GrabObject_Server`
  (params (Object :type "/Game/Core/Actor/BP_BaseGrapObject Object Reference"))
  (bind _returnvalue (`self.GetOwner`))
  (bind _staticmesh (`/Game/Core/Actor/BP_BaseObject.StaticMesh` (`self.HeldItem`)))
  ;[0.15 0.04532 0.02197 0.5] Server - Grab
  (`/Engine/EditorBlueprintResources/StandardMacros.IsValid` (`self.HeldItem`)
    (:`Is Not Valid`
      (if (and (`KismetSystemLibrary.IsValid` Object) (`KismetSystemLibrary.IsValid` _returnvalue))
        (bind _asbp_third_person_character (cast `/Game/ThirdPerson/Blueprints/BP_ThirdPersonCharacter` _returnvalue))
        (if (< (`Actor.GetDistanceTo` _asbp_third_person_character Object) 300.0)
          (set `/Game/Core/Actor/BP_BaseGrapObject.bIsHeld` true Object)
          (set `self.HeldItem` Object)
          (`Actor.SetOwner` (`self.HeldItem`) _asbp_third_person_character)
          (`PrimitiveComponent.SetSimulatePhysics` _staticmesh false)
          (`PrimitiveComponent.SetCollisionEnabled` _staticmesh "NoCollision")
          (`self.SetComponentTickEnabled` true)
          (bind _returnvalue_2 (`KismetSystemLibrary.K2_SetTimerDelegate` (delegate `Attach`) 0.02 true))
          (set `self.TimerHandle` _returnvalue_2))))))

(event `GrabObject`
  (params (Object :type "/Game/Core/Actor/BP_BaseGrapObject Object Reference"))
  ;[0.1343 0.15 0.003627 0.5] Client - Grab
  (`/Engine/EditorBlueprintResources/StandardMacros.IsValid` Object
    (:`Is Valid`
      (`/Engine/EditorBlueprintResources/StandardMacros.IsValid` (`self.HeldItem`)
        (:`Is Not Valid`
          (`self.GrabObject_Server` Object))))))

(event `Attach`
  ; Grab Attachment
  (`/Engine/EditorBlueprintResources/StandardMacros.IsValid` (`self.HeldItem`)
    (:`Is Valid`
      (`/Engine/EditorBlueprintResources/ActorComponentMacros.Switch Has Authority`
        (:`Authority`
          (bind _grabpoint (`/Game/ThirdPerson/Blueprints/BP_ThirdPersonCharacter.GrabPoint` (stale `GrabObject_Server` _asbp_third_person_character)))
          (bind _returnvalue (`SceneComponent.K2_GetComponentLocation` _grabpoint))
          (bind _returnvalue_2 (`KismetMathLibrary.VInterpTo` (`SceneComponent.K2_GetComponentLocation` (`/Game/Core/Actor/BP_BaseObject.StaticMesh` (`self.HeldItem`))) _returnvalue (`GameplayStatics.GetWorldDeltaSeconds`) 10.0))
          (`Actor.K2_SetActorLocation` (`self.HeldItem`) _returnvalue_2 false false)
          (if (< (`KismetMathLibrary.Vector_Distance` _returnvalue_2 _returnvalue) 5.0)
            (bind _returnvalue_3 (`Actor.K2_AttachToComponent` (`self.HeldItem`) _grabpoint "None" "SnapToTarget" "SnapToTarget" "SnapToTarget" true))
            (if _returnvalue_3
              (`KismetSystemLibrary.K2_ClearAndInvalidateTimerHandle` (`self.TimerHandle`)))))))))

(event `DropItem`
  (bind _helditem (`self.HeldItem`))
  (bind _staticmesh (`/Game/Core/Actor/BP_BaseObject.StaticMesh` (`self.HeldItem`)))
  ;[0.02643 0.1284 0.15 0.5] Drop Item- Detach
  (`KismetSystemLibrary.K2_ClearAndInvalidateTimerHandle` (`self.TimerHandle`))
  (`KismetSystemLibrary.PrintString` "geliyor mu yani")
  (`/Engine/EditorBlueprintResources/ActorComponentMacros.Switch Has Authority`
    (:`Authority`
      (`/Engine/EditorBlueprintResources/StandardMacros.IsValid` _helditem
        (:`Is Valid`
          (`Actor.K2_DetachFromActor` _helditem "KeepWorld" "KeepWorld" "KeepWorld")
          (`Actor.SetOwner` _helditem null)
          (`PrimitiveComponent.SetCollisionEnabled` _staticmesh "QueryAndPhysics")
          (`PrimitiveComponent.SetSimulatePhysics` _staticmesh true)
          (set `/Game/Core/Actor/BP_BaseGrapObject.bIsHeld` false (`self.HeldItem`))
          (set `self.HeldItem` null)
          (`self.SetComponentTickEnabled` false))
        (:`Is Not Valid`
          (`KismetSystemLibrary.PrintString` "mevcut değilll"))))
    (:`Remote`
      (`KismetSystemLibrary.PrintString` "bilemem"))))

(event `ServerDropItem`)

(fn `OnRep_HeldItem`)