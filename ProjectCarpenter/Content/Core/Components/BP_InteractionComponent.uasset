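; BP_InteractionComponent is an actor component that lets the third-person character interact with world objects or drop a held item.
; StartInteraction requests a drop if the grabbing component holds an item; otherwise it sphere-traces toward the control rotation for a BP_BaseObject, with debug drawing.
; Server events call InteractMessage on the hit actor or DropItem on the grabbing component.
; The interact event reads StartInteraction's trace result rather than receiving a target parameter.
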(event `StartInteraction`
  (bind _asbp_third_person_character (cast `/Game/ThirdPerson/Blueprints/BP_ThirdPersonCharacter` (`self.GetOwner`)))
  (`/Engine/EditorBlueprintResources/StandardMacros.IsValid` (`/Game/Core/Components/BP_GrabbingComponent.HeldItem` (`/Game/ThirdPerson/Blueprints/BP_ThirdPersonCharacter.BP_GrabbingComponent` _asbp_third_person_character))
    (:`Is Valid`
      ; Request Drop
      (`self.Server_RequestDropItem`))
    (:`Is Not Valid`
      (bind _returnvalue (`Actor.K2_GetActorLocation` _asbp_third_person_character))
      (bind (_outhit _returnvalue_2) (`KismetSystemLibrary.SphereTraceSingle` :`Start` _returnvalue :`End` (+ _returnvalue (* (`KismetMathLibrary.GetForwardVector` (`Pawn.GetControlRotation` _asbp_third_person_character)) 100.0)) :`Radius` 100.0 :`TraceChannel` "TraceTypeQuery1" :`DrawDebugType` "ForDuration"))
      (if _returnvalue_2
        (bind _asbp_base_object (cast `/Game/Core/Actor/BP_BaseObject` (`.HitActor` (`GameplayStatics.BreakHitResult` _outhit))))
        (`/Engine/EditorBlueprintResources/StandardMacros.IsValid` _asbp_base_object
          (:`Is Valid`
            (`self.TryInteraction`)))))))

(event `Interact_Server`
  ; Interaction Server
  (message `/Game/Core/Interfaces/BPI_Interact.Interact` (`.HitActor` (`GameplayStatics.BreakHitResult` (stale `StartInteraction` _outhit))) (stale `StartInteraction` _asbp_third_person_character)))

(event `TryInteraction`
  ; Interaction Server
  (`self.Interact_Server`))

(event `Server_RequestDropItem`
  (bind _returnvalue (`Actor.GetComponentByClass` (`self.GetOwner`) "/Game/Core/Components/BP_GrabbingComponent.BP_GrabbingComponent_C"))
  ; Drop Server
  (`/Engine/EditorBlueprintResources/StandardMacros.IsValid` _returnvalue
    (:`Is Valid`
      (`/Game/Core/Components/BP_GrabbingComponent.DropItem` _returnvalue))))

(event `RequestDropItem`
  ; Drop Server
  (`self.Server_RequestDropItem`))